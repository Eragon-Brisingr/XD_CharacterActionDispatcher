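; Example role actor that acts as a dispatcher holder and bridges action selections to an on-screen selection UI.
; On BeginPlay it creates the Example_UI_RoleSelections widget for player controller 0 and adds it to the viewport.
; Select, add and abort events reach the widget through Client-prefixed events, while a chosen option is forwarded to RoleSelection for execution.
; It stores the current main dispatcher, exposes its dispatcher list and always permits dispatcher execution.
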(event `self.ReceiveBeginPlay`
  (bind _returnvalue (`|CreateWidget` "/XD_CharacterActionDispatcher/UI/Example_UI_RoleSelections.Example_UI_RoleSelections_C" (`GameplayStatics.GetPlayerController` 0)))
  (bind _output_get (set `self.UI_RoleSelection` _returnvalue))
  (`UserWidget.AddToViewport` _output_get 0))

(event `XD_DispatchableEntityInterface.SetCurrentMainDispatcher`
  (params (Dispatcher :type "XD_ActionDispatcherBase Object Reference"))
  (set `self.MainDispatcher` Dispatcher))

(event `XD_DA_RoleSelectionInterface.ExecuteSelect`
  (params (RoleSelection :type "XD_DA_RoleSelectionBase Object Reference") (Selections :type "Array of DA_DisplaySelection Structure (by ref)"))
  (`self.ClientShowSelection` Selections))

(event `XD_DA_RoleSelectionInterface.WhenSelected`
  (params (Selection :type "DA_DisplaySelection Structure (by ref)"))
  (`self.ClientWhenSelected` Selection))

(event `ClientShowSelection`
  (params (Selections :type "Array of DA_DisplaySelection Structure (by ref)"))
  (`/XD_CharacterActionDispatcher/UI/Example_UI_RoleSelections.ShowSelections` (`self.UI_RoleSelection`) Selections))

(event `ClientWhenSelected`
  (params (Selection :type "DA_DisplaySelection Structure (by ref)"))
  (`XD_DA_RoleSelectionBase.ExecuteSelection` (stale `XD_DA_RoleSelectionInterface.ExecuteSelect` RoleSelection) Selection))

(event `XD_DA_RoleSelectionInterface.ExecuteAddSelects`
  (params (Selections :type "Array of DA_DisplaySelection Structure (by ref)"))
  (`self.ClientShowSelection` Selections))

(event `XD_DA_RoleSelectionInterface.ExecuteAbortSelect`
  (`self.ClientAbortSelect`))

(event `ClientAbortSelect`
  (`/XD_CharacterActionDispatcher/UI/Example_UI_RoleSelections.WhenAbortSelection` (`self.UI_RoleSelection`)))

(fn `CanExecuteDispatcher`
  (returns (ReturnValue :type Boolean))
  (return true))

(fn `GetCurrentDispatchableActions`
  (returns (ReturnValue :type "XD_DispatchableActionList Structure"))
  (return (make `XD_DispatchableActionList` (`self.Dispatchers`))))

(fn `GetCurrentMainDispatcher`
  (returns (ReturnValue :type "XD_ActionDispatcherBase Object Reference"))
  (return (`self.MainDispatcher`)))

(fn `UserConstructionScript`)