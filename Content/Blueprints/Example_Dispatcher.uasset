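; Example dispatcher that demonstrates launching dispatchable actions from the WhenDispatchStart event.
; On start, a Sequence issues four XD_DA_Exmaple actions back to back, each with its own delay time.
; An unconnected branch sketches a FlowControlTogether join: two pawns run MoveTo actions and report arrival to a flow control, whose Together output plays a level sequence.
; That branch also prints debug text for the join and its numbered waiting states, but never runs.
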(event `self.WhenDispatchStart`
  (`|ExecutionSequence`
    (:`then_0`
      (`|ExecuteAction` "/Script/XD_CharacterActionDispatcher.XD_DA_Exmaple" 2.0))
    (:`then_1`
      (`|ExecuteAction` "/Script/XD_CharacterActionDispatcher.XD_DA_Exmaple" 4.0))
    (:`then_2`
      (`|ExecuteAction` "/Script/XD_CharacterActionDispatcher.XD_DA_Exmaple" 3.0))
    (:`then_3`
      (`|ExecuteAction` "/Script/XD_CharacterActionDispatcher.XD_DA_Exmaple" 1.0))))